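; BP_PlayerController is a player controller that drives movement of a top-down camera pawn.
; On BeginPlay it adds the IMC_CameraMove Enhanced Input mapping context, shows the mouse cursor and caches the BP_TopDownCamera pawn and its movement component.
; The IA_Move action passes its X and Y axis values to that component's BasicMovementControls, leaving the movement logic to the pawn's component.
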(event Input|EnhancedActionEvents|EnhancedInputActionIA_Move
  (params (ActionValue :type Vector%202D%20Structure) (ElapsedSeconds :type Float%20%28double-precision%29) (TriggeredSeconds :type Float%20%28double-precision%29) (InputAction :type Input%20Action%20Object%20Reference :default "/Game/Blueprints/IA_Move.IA_Move"))
  (:Triggered
    (Default|BasicMovementControls (Variables|Default|GetCameraMovementRef) (.x ActionValue) (.y ActionValue))))

(event EventBeginPlay
  (Utilities|FlowControl|Sequence
    (:then_0
      (Input|AddMappingContext (PlayerController|LocalPlayerSubsystems|GetEnhancedInputLocalPlayerSubsystem) "/Game/Blueprints/IMC_CameraMove.IMC_CameraMove" 0 "(bIgnoreAllPressedKeysUntilRelease=True,bForceImmediately=False,bNotifyUserSettings=False)")
      (Variables|Default|SetbShowMouseCursor true)
      (bind _asbp_top_down_camera (Utilities|Casting|CastToBP_TopDownCamera (Game|Player|GetPlayerPawn 0)))
      (bind _output_get (Variables|References|SetCameraPawnRef _asbp_top_down_camera))
      (Variables|Default|SetCameraMovementRef (Variables|/Game/Blueprints/BP_TopDownCamera.BP_TopDownCamera_C|GetPawnMovementComponent _output_get)))))

(event EventTick
  (params (DeltaSeconds :type Float%20%28single-precision%29)))

(fn ConstructionScript)