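; Movement component for the top-down camera pawn that pans it from two input axis values.
; It caches its owning BP_TopDownCamera on component init.
; BasicMovementControls offsets the pawn in local space on X, Y or both, scaled by default speed and a speed modifier, unless camera movement is disabled.
; Movement has no sweep or delta-time scaling, so speed depends on how often it is called.
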(event Custom|InitComponent
  ;[0.15 0.15 0.15 0.5] Gets hard reference to camera pawn
  (bind _asbp_top_down_camera (Utilities|Casting|CastToBP_TopDownCamera (Components|GetOwner)))
  (Variables|References|SetCameraPawnRef _asbp_top_down_camera))

(event EventBeginPlay)

(event EventTick
  (params (DeltaSeconds :type Float%20%28single-precision%29)))

(fn BasicMovementControls
  (params (AxisValueX :type Float%20%28double-precision%29) (AxisValueY :type Float%20%28double-precision%29))
  (LocalVariables|SetAxisValueXLocal AxisValueX)
  (LocalVariables|SetAxisValueYLocal AxisValueY)
  (if (not (Variables|Movement|Bools|GetbDisableCameraMovement))
    ;[0.15 0.15 0.15 0.5] Both X and Y
    (if (and (!= (LocalVariables|GetAxisValueXLocal) 0.0) (!= (LocalVariables|GetAxisValueYLocal) 0.0))
      (Transformation|AddActorLocalOffset (Variables|References|GetCameraPawnRef) (+ (Math|Vector|MakeVector (* (LocalVariables|GetAxisValueXLocal) (Variables|Movement|Settings|GetDefaultMovementSpeed) (Variables|Movement|Settings|GetMovementSpeedModifier)) 0.0 0.0) (Math|Vector|MakeVector 0.0 (* (LocalVariables|GetAxisValueYLocal) (Variables|Movement|Settings|GetDefaultMovementSpeed) (Variables|Movement|Settings|GetMovementSpeedModifier)) 0.0)) false false)
      (else
        ;[0.15 0.15 0.15 0.5] Just X
        (if (!= (LocalVariables|GetAxisValueXLocal) 0.0)
          (Transformation|AddActorLocalOffset (Variables|References|GetCameraPawnRef) (Math|Vector|MakeVector (* (LocalVariables|GetAxisValueXLocal) (Variables|Movement|Settings|GetDefaultMovementSpeed) (Variables|Movement|Settings|GetMovementSpeedModifier)) 0.0 0.0) false false)
          (else
            ;[0.15 0.15 0.15 0.5] Just Y
            (if (!= (LocalVariables|GetAxisValueYLocal) 0.0)
              (Transformation|AddActorLocalOffset (Variables|References|GetCameraPawnRef) (Math|Vector|MakeVector 0.0 (* (LocalVariables|GetAxisValueYLocal) (Variables|Movement|Settings|GetDefaultMovementSpeed) (Variables|Movement|Settings|GetMovementSpeedModifier)) 0.0) false false))))))))